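; Hands-and-controllers component for VR that extends its parent with grab action input for BP_HAC_GS hand actors.
; SpawnHACGSs spawns left and right hand actors from the supplied mesh, visibility and optimization settings, snaps them to their roots and enables the laser on the right.
; Boolean, float, 2D and Cap controller input overrides forward each event to the matching hand's GrabActionKey function, then call the parent implementation.
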(event EventBeginPlay
  (|CallParentFunction) ; This node is disabled and will not be called.\nDrag off pins to build functionality.
)

(event EventTick
  (params (DeltaSeconds :type Float%20%28single-precision%29))
  (|CallParentFunction DeltaSeconds) ; This node is disabled and will not be called.\nDrag off pins to build functionality.
)

(fn ControllerInput(Boolean)
  (params (Hand :type E_Hand%20Enum :default "NewEnumerator0") (Button :type E_ControllerButtons_Boolean%20Enum :default "NewEnumerator0") (Pressed :type Boolean))
  (Default|GrabActionKey(Boolean) (Setup|GetHandGS Hand) Button Pressed)
  (|CallParentFunction Hand Button Pressed))

(fn ControllerInput(Float)
  (params (Hand :type E_Hand%20Enum :default "NewEnumerator0") (Button :type E_ControllerButtons_Float%20Enum :default "NewEnumerator4") (Axis :type Float%20%28single-precision%29))
  (Default|GrabActionKey(Float) (Setup|GetHandGS Hand) Button Axis)
  (|CallParentFunction Hand Button Axis))

(fn ControllerInput(2D)
  (params (Hand :type E_Hand%20Enum :default "NewEnumerator0") (Button :type E_ControllerButtons_2D%20Enum :default "NewEnumerator7") (2D :type Vector%202D%20Structure))
  (Default|GrabActionKey(2D) (Setup|GetHandGS Hand) Button 2D)
  (|CallParentFunction Hand Button 2D))

(fn ControllerInput(Cap)
  (params (Hand :type E_Hand%20Enum :default "NewEnumerator0") (Button :type E_ControllerButtons_Cap%20Enum :default "NewEnumerator0") (Cap :type Boolean))
  (Default|GrabActionKey(Cap) (Setup|GetHandGS Hand) Button Cap)
  (|CallParentFunction Hand Button Cap))

(fn SpawnHACGSs
  (params (Settings :type S%20Settings%20Structure%20%28by%20ref%29) (LeftRoot :type Scene%20Component%20Object%20Reference) (RightRoot :type Scene%20Component%20Object%20Reference))
  (bind (_controllermesh _handmesh _visibility _optimized) (Utilities|Struct|BreakS_Settings Settings))
  (bind _returnvalue (Components|GetOwner))
  (bind _returnvalue_2 (Math|Transform|MakeTransform "0, 0, 0"))
  (bind _returnvalue_3 (Game|SpawnActorfromClass "/Game/VRImmersiveHands/HandsAndControllers/Blueprints/BP_HAC_GS.BP_HAC_GS_C" _returnvalue_2 "AlwaysSpawn" _returnvalue "NewEnumerator0" _controllermesh _handmesh _visibility _optimized false 0))
  (bind _output_get (Variables|Default|SetLeftHAC _returnvalue_3))
  (Transformation|AttachComponentToComponent _output_get LeftRoot "None" "SnapToTarget" "SnapToTarget" "KeepWorld" true)
  (bind _returnvalue_4 (Game|SpawnActorfromClass "/Game/VRImmersiveHands/HandsAndControllers/Blueprints/BP_HAC_GS.BP_HAC_GS_C" _returnvalue_2 "AlwaysSpawn" _returnvalue "NewEnumerator1" _controllermesh _handmesh _visibility _optimized true 0))
  (bind _output_get_2 (Variables|Default|SetRightHAC _returnvalue_4))
  (Transformation|AttachComponentToComponent _output_get_2 RightRoot "None" "SnapToTarget" "SnapToTarget" "KeepWorld" true)
  (return _returnvalue_3 _returnvalue_4))

(fn GetHandGS
  (params (Hand :type E_Hand%20Enum :default "NewEnumerator0"))
  (return (.AsBP%20HAC%20GS (Utilities|Casting|CastToBP_HAC_GS (CallFunction|GetHand Hand)))))