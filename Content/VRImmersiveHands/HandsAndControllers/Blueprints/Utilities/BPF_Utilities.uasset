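; Blueprint function library of shared VR helpers for the hands and controllers system.
; It detects the headset and its DOF, toggles stereo rendering, plays haptics and fetches left and right HACs from the player pawn's BPAC_HAC.
; It also inverts and mirrors hand transforms, auto-scrolls hovered BPI_UI widgets outside a center dead zone, and logs to BPW_Console.
; Tag helpers store key-value pairs as adjacent array entries.
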(fn AutoDetectHMD
  (switch string (Utilities|String|ToString(Name) (Class|HeadMountedDisplayFunctionLibrary|GetHMDDeviceName))
    (:Default
      _)
    (:SteamVR
      (switch string ""
        (:Default
          _)
        (:Valve%20Index
          (LocalVariables|SetTemp "NewEnumerator5")
          (return true (LocalVariables|GetTemp)))
        (:Vive
          (LocalVariables|SetTemp "NewEnumerator0" :!label _label)
          (return true (LocalVariables|GetTemp)))
        (:Vive%20Pro
          (goto _label))
        (:Vive%20Cosmos
          (LocalVariables|SetTemp "NewEnumerator9")
          (return true (LocalVariables|GetTemp)))))
    (:OculusHMD
      (switch string (Class|OculusFunctionLibrary|GetDeviceName)
        (:Default
          _)
        (:Oculus%20Rift
          (LocalVariables|SetTemp "NewEnumerator1")
          (return true (LocalVariables|GetTemp)))
        (:Oculus%20Go
          (LocalVariables|SetTemp "NewEnumerator2")
          (return true (LocalVariables|GetTemp)))
        (:Oculus%20Quest
          (LocalVariables|SetTemp "NewEnumerator3" :!label _label_2)
          (return true (LocalVariables|GetTemp)))
        (:Oculus%20Rift%20S
          (goto _label_2))
        (:Oculus%20Unknown
          (LocalVariables|SetTemp "NewEnumerator8")
          (return true (LocalVariables|GetTemp)))))
    (:WindowsMixedRealityHMD
      (LocalVariables|SetTemp "NewEnumerator7")
      (return true (LocalVariables|GetTemp))))
  (return false "NewEnumerator4"))

(fn GetDOF
  (params (HMD :type E_HMD%20Enum :default "NewEnumerator4"))
  (return (Utilities|Select :Index HMD :NewEnumerator4 "NewEnumerator0" :NewEnumerator5 "NewEnumerator1" :NewEnumerator0 "NewEnumerator1" :NewEnumerator9 "NewEnumerator1" :NewEnumerator1 "NewEnumerator1" :NewEnumerator2 "NewEnumerator0" :NewEnumerator3 "NewEnumerator1" :NewEnumerator6 "NewEnumerator1" :NewEnumerator8 "NewEnumerator0" :NewEnumerator7 "NewEnumerator1")))

(fn EnableVR
  (params (Enable :type Boolean) (PixelDensity :type Float%20%28single-precision%29))
  (if Enable
    (Development|ExecuteConsoleCommand 0 (Utilities|String|Append "vr.PixelDensity " (Utilities|String|ToString(Float) PixelDensity)) 0)
    (Class|HeadMountedDisplayFunctionLibrary|EnableHMD true)
    (Development|ExecuteConsoleCommand 0 "vr.bEnableStereo True" 0)
    (else
      (Class|HeadMountedDisplayFunctionLibrary|EnableHMD false)
      (Development|ExecuteConsoleCommand 0 "vr.bEnableStereo False" 0))))

(fn Rumble
  (params (Both :type Boolean) (Hand :type E_Hand%20Enum :default "NewEnumerator0") (Intensity :type Float%20%28single-precision%29) (HapticEffect :type Haptic%20Feedback%20Effect%20Base%20Object%20Reference))
  (bind _returnvalue (Game|GetPlayerController 0))
  (bind _returnvalue_2 (Utilities|Select :Index Hand :NewEnumerator0 "Left" :NewEnumerator1 "Right"))
  (if Both
    (Class|PlayerController|PlayHapticEffect _returnvalue HapticEffect _returnvalue_2 Intensity false)
    (else
      (Class|PlayerController|PlayHapticEffect _returnvalue HapticEffect _returnvalue_2 Intensity false))))

(fn GetBPACHAC
  (bind _returnvalue (Game|Player|GetPlayerPawn 0))
  (bind _returnvalue_2 (Actor|GetComponentbyClass _returnvalue "/Game/VRImmersiveHands/HandsAndControllers/Blueprints/BPAC_HAC.BPAC_HAC_C"))
  (Utilities|IsValid _returnvalue_2
    (:Is%20Valid
      (return true _returnvalue_2))
    (:Is%20Not%20Valid
      (return false 0))))

(fn GetHACs
  (bind (_bsuccess _component) (GetRef|GetBPACHAC))
  (if _bsuccess
    (return true (Variables|/Game/VRImmersiveHands/HandsAndControllers/Blueprints/BPAC_HAC.BPAC_HAC_C|GetLeftHAC _component) (Variables|/Game/VRImmersiveHands/HandsAndControllers/Blueprints/BPAC_HAC.BPAC_HAC_C|GetRightHAC _component))
    (else
      (return false 0 0))))

(fn GetHAC
  (params (Hand :type E_Hand%20Enum :default "NewEnumerator0"))
  (bind (_bsuccess _left _right) (GetRef|GetHACs))
  (if _bsuccess
    (return _bsuccess (Utilities|Select :Index Hand :NewEnumerator0 _left :NewEnumerator1 _right) (Utilities|Select :Index Hand :NewEnumerator0 _right :NewEnumerator1 _left))
    (else
      (return false 0 0))))

(fn PrinttoConsole
  (params (InText :type Text) (Color :type Linear%20Color%20Structure :default "(R=1.000000,G=1.000000,B=1.000000,A=1.000000)"))
  (Development|PrintString 0 (Utilities|String|ToString(Text) InText) true true Color)
  (bind _outactors (Actor|GetAllActorsOfClass 0 "/Game/VRImmersiveHands/Pawn/Blueprints/BPW_Console.BPW_Console_C"))
  (if (Utilities|Array|IsValidIndex _outactors)
    (Default|PrintString (Variables|/Game/VRImmersiveHands/Pawn/Blueprints/BPW_Console.BPW_Console_C|GetRef (Utilities|Array|Get(acopy) _outactors)) InText Color)))

(fn PrinttoConsoleW/Ref
  (params (Ref :type BPW%20Console%20Object%20Reference) (InText :type Text) (Color :type Linear%20Color%20Structure :default "(R=1.000000,G=1.000000,B=1.000000,A=1.000000)"))
  (Development|PrintString 0 (Utilities|String|ToString(Text) InText) true true Color)
  (Utilities|IsValid Ref
    (:Is%20Valid
      (Default|PrintString (Variables|/Game/VRImmersiveHands/Pawn/Blueprints/BPW_Console.BPW_Console_C|GetRef Ref) InText Color))))

(fn AutoScroll
  (params (WidgetInteraction :type Widget%20Interaction%20Component%20Object%20Reference) (DeadZoneRatio :type Float%20%28single-precision%29) (Sensetivity :type Float%20%28single-precision%29))
  (bind _returnvalue (Class|WidgetInteractionComponent|GetHoveredWidgetComponent WidgetInteraction))
  (bind _returnvalue_2 (Class|WidgetInteractionComponent|Get2DHitLocation WidgetInteraction))
  (bind _returnvalue_3 (UserInterface|GetUserWidgetObject _returnvalue))
  (Utilities|IsValid _returnvalue
    (:Is%20Valid
      (if (Utilities|DoesObjectImplementInterface _returnvalue_3 "/Game/VRImmersiveHands/HandsAndControllers/Blueprints/Utilities/BPI_UI.BPI_UI_C")
        (bind (_res _vertical) (Class|BPIUI|GetSize(Message) _returnvalue_3))
        (Utilities|IsValid WidgetInteraction
          (:Is%20Valid
            (LocalVariables|SetAutoScrollValue (select _vertical (.y _returnvalue_2) (.x _returnvalue_2)))
            (if (not (Math|Float|InRange(Float) (LocalVariables|GetAutoScrollValue) (- (/ (select _vertical (.Y (Math|Vector2D|BreakVector2D _res)) (.X (Math|Vector2D|BreakVector2D _res))) 2.0) (* (/ (select _vertical (.Y (Math|Vector2D|BreakVector2D _res)) (.X (Math|Vector2D|BreakVector2D _res))) 2.0) DeadZoneRatio)) (+ (/ (select _vertical (.Y (Math|Vector2D|BreakVector2D _res)) (.X (Math|Vector2D|BreakVector2D _res))) 2.0) (* (/ (select _vertical (.Y (Math|Vector2D|BreakVector2D _res)) (.X (Math|Vector2D|BreakVector2D _res))) 2.0) DeadZoneRatio))))
              (Math|Float|CompareFloat (LocalVariables|GetAutoScrollValue) (/ (select _vertical (.Y (Math|Vector2D|BreakVector2D _res)) (.X (Math|Vector2D|BreakVector2D _res))) 2.0)
                (:>
                  (Class|WidgetInteractionComponent|ScrollWheel WidgetInteraction (* (/ (Math|Float|Absolute(Float) (- (LocalVariables|GetAutoScrollValue) (+ (/ (select _vertical (.Y (Math|Vector2D|BreakVector2D _res)) (.X (Math|Vector2D|BreakVector2D _res))) 2.0) (* (/ (select _vertical (.Y (Math|Vector2D|BreakVector2D _res)) (.X (Math|Vector2D|BreakVector2D _res))) 2.0) DeadZoneRatio)))) Sensetivity) -1.0)))
                (:<
                  (Class|WidgetInteractionComponent|ScrollWheel WidgetInteraction (/ (Math|Float|Absolute(Float) (- (LocalVariables|GetAutoScrollValue) (- (/ (select _vertical (.Y (Math|Vector2D|BreakVector2D _res)) (.X (Math|Vector2D|BreakVector2D _res))) 2.0) (* (/ (select _vertical (.Y (Math|Vector2D|BreakVector2D _res)) (.X (Math|Vector2D|BreakVector2D _res))) 2.0) DeadZoneRatio)))) Sensetivity)))))))))))

(fn GetHandTransform
  (params (Transform :type Transform) (Inverted :type Boolean) (HandScale :type Float%20%28single-precision%29))
  (bind _returnvalue (/ 1.0 HandScale))
  (bind _returnvalue_2 (Math|Conversions|ToVector(Float) _returnvalue))
  (bind _returnvalue_3 (Math|Transform|InvertTransform (Math|Transform|MakeTransform (.location Transform) (.rotation Transform) _returnvalue_2)))
  (if Inverted
    (return (Math|Transform|MakeTransform (* (.location _returnvalue_3) "1.000000,-1.000000,1.000000") (Math|Rotator|MakeRotator (* (.roll (.rotation _returnvalue_3)) -1.0) (.pitch (.rotation _returnvalue_3)) (* (.yaw (.rotation _returnvalue_3)) -1.0)) (* (.scale _returnvalue_3) "1.000000,-1.000000,1.000000")))
    (else
      (return (Math|Transform|InvertTransform (Math|Transform|MakeTransform (.location Transform) (.rotation Transform) _returnvalue_2))))))

(fn GetTagValue
  (params (Tags :type Array%20of%20Names) (Tag :type Name))
  (bind _returnvalue (Utilities|Array|FindItem Tags Tag))
  (if (not (== _returnvalue -1))
    (return true (Utilities|Array|Get(acopy) Tags (+ _returnvalue 1)))
    (else
      (return false "None"))))

(fn SetTagValue
  (params (Tags :type Array%20of%20Names) (Tag :type Name) (Value :type Name))
  (Utilities|Array|Add Tags Tag)
  (Utilities|Array|Add Tags Value))

(fn PrintWarning
  (params (Error :type Boolean) (Reason :type String))
  (Console|PrinttoConsole (Utilities|Text|ToText(String) (Utilities|String|Append (select Error "ERROR:: " "WARNING:: ") Reason)) (Math|Color|SelectColor "(R=1.000000,G=0.082165,B=0.062269,A=1.000000)" "(R=1.000000,G=0.926902,B=0.020833,A=1.000000)" Error)))