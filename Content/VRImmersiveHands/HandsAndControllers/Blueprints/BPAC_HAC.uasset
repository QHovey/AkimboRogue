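; Actor component that manages the left and right VR hand-and-controller actors (BP_HAC) for its owner.
; SpawnHACs spawns both from a settings struct and attaches them to the supplied roots, with the laser set on the right.
; Typed input functions route button, axis, 2D and capacitive-touch values to the chosen hand through GetHand.
; Other functions forward widget selection, emotes, laser toggling and selective runtime updates of meshes, visibility and optimization.
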(event EventBeginPlay)

(event EventTick
  (params (DeltaSeconds :type Float%20%28single-precision%29)))

(fn SpawnHACs
  (params (Settings :type S%20Settings%20Structure) (LeftRoot :type Scene%20Component%20Object%20Reference) (RightRoot :type Scene%20Component%20Object%20Reference))
  (bind (_controllermesh _handmesh _visibility _optimized) (Utilities|Struct|BreakS_Settings Settings))
  (bind _returnvalue (Components|GetOwner))
  (bind _returnvalue_2 (Math|Transform|MakeTransform "0, 0, 0"))
  (bind _returnvalue_3 (Game|SpawnActorfromClass "/Game/VRImmersiveHands/HandsAndControllers/Blueprints/BP_HAC.BP_HAC_C" _returnvalue_2 "AlwaysSpawn" _returnvalue "NewEnumerator0" _controllermesh _handmesh _visibility _optimized false 0))
  (bind _output_get (Variables|ForInternalUse!|SetLeftHAC _returnvalue_3))
  (Transformation|AttachComponentToComponent _output_get LeftRoot "None" "SnapToTarget" "SnapToTarget" "KeepWorld" true)
  (bind _returnvalue_4 (Game|SpawnActorfromClass "/Game/VRImmersiveHands/HandsAndControllers/Blueprints/BP_HAC.BP_HAC_C" _returnvalue_2 "AlwaysSpawn" _returnvalue "NewEnumerator1" _controllermesh _handmesh _visibility _optimized true 0))
  (bind _output_get_2 (Variables|ForInternalUse!|SetRightHAC _returnvalue_4))
  (Transformation|AttachComponentToComponent _output_get_2 RightRoot "None" "SnapToTarget" "SnapToTarget" "KeepWorld" true)
  (return (Variables|ForInternalUse!|GetLeftHAC) (Variables|ForInternalUse!|GetRightHAC)))

(fn ControllerInput(Boolean)
  (params (Hand :type E_Hand%20Enum :default "NewEnumerator0") (Button :type E_ControllerButtons_Boolean%20Enum :default "NewEnumerator0") (Pressed :type Boolean))
  (bind _ref (Setup|GetHand Hand))
  (switch Utilities|FlowControl|Switch|SwitchonE_ControllerButtons_Boolean Button
    (:NewEnumerator0
      (Default|UpdateButton1 _ref Pressed))
    (:NewEnumerator1
      (Default|UpdateButton2 _ref Pressed))
    (:NewEnumerator2
      (Default|UpdateSystem _ref Pressed))
    (:NewEnumerator3
      (Default|UpdateMenu _ref Pressed))
    (:NewEnumerator5
      (Default|UpdateShoulder _ref Pressed))))

(fn ControllerInput(Float)
  (params (Hand :type E_Hand%20Enum :default "NewEnumerator0") (Button :type E_ControllerButtons_Float%20Enum :default "NewEnumerator4") (Axis :type Float%20%28single-precision%29))
  (bind _ref (Setup|GetHand Hand))
  (switch Utilities|FlowControl|Switch|SwitchonE_ControllerButtons_Float Button
    (:NewEnumerator4
      (Default|UpdateTrigger _ref Axis))
    (:NewEnumerator6
      (Default|UpdateGrip _ref Axis))))

(fn ControllerInput(2D)
  (params (Hand :type E_Hand%20Enum :default "NewEnumerator0") (Button :type E_ControllerButtons_2D%20Enum :default "NewEnumerator7") (2D :type Vector%202D%20Structure))
  (bind _ref (Setup|GetHand Hand))
  (switch Utilities|FlowControl|Switch|SwitchonE_ControllerButtons_2D Button
    (:NewEnumerator7
      (Default|UpdateStick2D _ref 2D))
    (:NewEnumerator8
      (Default|UpdatePad2D _ref 2D))))

(fn ControllerInput(Cap)
  (params (Hand :type E_Hand%20Enum :default "NewEnumerator0") (Button :type E_ControllerButtons_Cap%20Enum :default "NewEnumerator0") (Cap :type Boolean))
  (bind _ref (Setup|GetHand Hand))
  (switch Utilities|FlowControl|Switch|SwitchonE_ControllerButtons_Cap Button
    (:NewEnumerator0
      (Default|UpdateButton1Cap _ref Cap))
    (:NewEnumerator1
      (Default|UpdateButton2Cap _ref Cap))
    (:NewEnumerator2
      (Default|UpdateSystemCap _ref Cap))
    (:NewEnumerator4
      (Default|UpdateTriggerCap _ref Cap))
    (:NewEnumerator7
      (Default|UpdateStickCap _ref Cap))
    (:NewEnumerator8
      (Default|UpdatePadCap _ref Cap))))

(fn WidgetInteract
  (params (Hand :type E_Hand%20Enum :default "NewEnumerator0") (Select :type Boolean))
  (bind _ref (Setup|GetHand Hand))
  (if Select
    (Default|WidgetSelect _ref)
    (else
      (Default|WidgetDeselect _ref))))

(fn UpdateLaser
  (params (Hand :type E_Hand%20Enum :default "NewEnumerator0") (Laser :type Boolean))
  (Variables|/Game/VRImmersiveHands/HandsAndControllers/Blueprints/BP_HAC.BP_HAC_C|SetLaser (Setup|GetHand Hand) Laser))

(fn UpdateHAC
  (params (Hand :type E_Hand%20Enum :default "NewEnumerator0") (UpdateController :type Boolean) (ControllerMesh :type E_HMD%20Enum :default "NewEnumerator3") (UpdateHand :type Boolean) (HandMesh :type E_HandMeshes%20Enum :default "NewEnumerator0") (UpdateVisibility :type Boolean) (Visibility :type E_HACVisibility%20Enum :default "NewEnumerator2") (UpdateOptimization :type Boolean) (Optimization :type E_Optimization%20Enum :default "NewEnumerator2"))
  (bind _ref (Setup|GetHand Hand))
  (Default|UpdateHAC _ref (select UpdateController ControllerMesh (Variables|/Game/VRImmersiveHands/HandsAndControllers/Blueprints/BP_HAC.BP_HAC_C|GetControllerMesh _ref)) (select UpdateHand HandMesh (Variables|/Game/VRImmersiveHands/HandsAndControllers/Blueprints/BP_HAC.BP_HAC_C|GetHandMesh _ref)) (select UpdateVisibility Visibility (Variables|/Game/VRImmersiveHands/HandsAndControllers/Blueprints/BP_HAC.BP_HAC_C|GetVisibility _ref)) (select UpdateOptimization Optimization (Variables|/Game/VRImmersiveHands/HandsAndControllers/Blueprints/BP_HAC.BP_HAC_C|GetOptimization _ref))))

(fn GetHand
  (params (Hand :type E_Hand%20Enum :default "NewEnumerator0"))
  (return (Utilities|Select :Index Hand :NewEnumerator0 (Variables|ForInternalUse!|GetLeftHAC) :NewEnumerator1 (Variables|ForInternalUse!|GetRightHAC))))

(fn Emote
  (params (Hand :type E_Hand%20Enum :default "NewEnumerator0") (Anim :type Anim%20Sequence%20Object%20Reference))
  (Default|HandEmote (Setup|GetHand Hand) true Anim))

(fn ClearEmote
  (params (Hand :type E_Hand%20Enum :default "NewEnumerator0"))
  (Default|HandEmote (Setup|GetHand Hand) false))