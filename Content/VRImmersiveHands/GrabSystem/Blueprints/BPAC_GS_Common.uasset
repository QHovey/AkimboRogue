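; Common actor component for the VR hands grab system, providing setup and lookup helpers on its owner.
; InitializeComponent finds a mesh by tag, falling back to the owner's first mesh with a warning.
; GetGrabbingCore caches the owner's BPAC_GS_Core, or self-destructs through DestroyComponent if it is missing or being destroyed, calling CallOnDestroy first.
; Warnings are prefixed with the owning actor's name and can be muted with SupressWarnings.
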(fn InitializeComponent
  (params (Tag :type Name))
  (bind (_success _meshcomponent) (Core|FindMeshinOwner Tag))
  (if _success
    (return true _meshcomponent)
    (else
      (bind (_success_2 _meshcomponent_2) (Core|GetFirstMeshinOwner))
      (if _success_2
        (Utilities|PrintWarning false (Utilities|String|Append "Couldn't find a mesh component with the following tag, --- " (Utilities|String|ToString(Name) Tag) " ---. " (Utilities|GetObjectName _meshcomponent_2) " will be used instead."))
        (return true _meshcomponent_2)
        (else
          (return false 0))))))

(fn FindMeshinOwner
  (params (Tag :type Name))
  (LocalVariables|SetMesh 0)
  (bind _array_element (Utilities|Array|ForEachLoopwithBreak (Actor|GetComponentsByClass (Components|GetOwner) "/Script/Engine.MeshComponent") :!label _label)
    (:LoopBody
      (if (Utilities|Array|ContainsItem (Variables|/Script/Engine.ActorComponent|GetComponentTags _array_element) Tag)
        (LocalVariables|SetMesh _array_element)
        (goto _label Break)))
    (:Completed
      (bind _mesh (LocalVariables|GetMesh)
        (:then
          (return true _mesh))
        (:else
          (return false 0))))))

(fn GetFirstMeshinOwner
  (bind _output_get (LocalVariables|SetMesh (Actor|GetComponentbyClass (Components|GetOwner) "/Script/Engine.MeshComponent")))
  (Utilities|IsValid _output_get
    (:Is%20Valid
      (return true _output_get))
    (:Is%20Not%20Valid
      (return false 0))))

(fn DestroyComponent
  (params (Reason :type String))
  (Default|CallOnDestroy)
  (Utilities|PrintWarning true (Utilities|String|Append Reason " Destroying ---" (Utilities|GetDisplayName self) "---"))
  (Components|DestroyComponent))

(fn FindComponent
  (params (ComponentClass :type BPAC%20GS%20Common%20Class%20Reference))
  (bind _returnvalue (Components|GetOwner))
  (bind _returnvalue_2 (Actor|GetComponentbyClass _returnvalue ComponentClass))
  (Utilities|IsValid _returnvalue_2
    (:Is%20Valid
      (return true _returnvalue_2))
    (:Is%20Not%20Valid
      (return false 0))))

(fn GetGrabbingCore
  (bind _component (Core|FindComponent "/Game/VRImmersiveHands/GrabSystem/Blueprints/BPAC_GS_Core.BPAC_GS_Core_C"))
  (bind _asbpac_gs_core (Utilities|Casting|CastToBPAC_GS_Core _component)
    (:then
      (bind _output_get (Variables|ForInternalUse!|SetGrabbingCore _asbpac_gs_core))
      (if (Class|ActorComponent|IsBeingDestroyed _output_get)
        (Utilities|DestroyComponent "BPAC_GS_Core is being destroyed.")
        (return false 0)
        (else
          (return true _output_get))))
    (:CastFailed
      (Utilities|DestroyComponent "Couldn't find BPAC_GS_Core in the parent.")
      (return false 0))))

(fn PrintWarning
  (params (Error :type Boolean) (Reason :type String))
  (if (not (Variables|Settings|GetSupressWarnings))
    (CallFunction|PrintWarning Error (Utilities|String|Append "Actor --- " (Utilities|GetDisplayName (Components|GetOwner)) " --- " Reason))))