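; Child-actor helper that defines VR hand grab points on the actor containing it.
; Its construction script previews each point with an optional billboard and posed hand meshes on the parent actor, including inverted variants.
; Setup adds a sphere component per point to the attach parent, encoding grab type, index, priority and secondary-only flag as component tags.
; SetupGPC feeds it the actor's own GrabPoints, while SetupGSC accepts an external array.
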(event EventBeginPlay)

(fn ConstructionScript
  (bind _pointsize (Variables|Grab|GetPointSize))
  (bind _handscale (Variables|Grab|Preview|GetHandScale))
  (if (Class|Actor|IsChildActor)
    (Transformation|ResetRelativeTransform (Class|Actor|GetParentComponent))
    ;[1 1 1] Preview
    (for _array_element (Variables|Grab|GetGrabPoints)
      (if (Variables|Grab|GetPointPreview)
        (bind _returnvalue (AddComponent|AddBillboardComponent false (Math|Transform|MakeTransform (.GrabPoint (Utilities|Struct|BreakS_GrabPoints _array_element)) "0, 0, 0" "1,1,1")))
        (Rendering|Components|Sprite|SetSprite _returnvalue (Utilities|Select :Index (.GrabType (Utilities|Struct|BreakS_GrabPoints _array_element)) :NewEnumerator0 (Utilities|Select :Index _pointsize :Option%200 0 :Option%201 "/Game/VRImmersiveHands/GrabSystem/Textures/T_GrabPoint_64.T_GrabPoint_64" :Option%202 "/Game/VRImmersiveHands/GrabSystem/Textures/T_GrabPoint_128.T_GrabPoint_128" :Option%203 "/Game/VRImmersiveHands/GrabSystem/Textures/T_GrabPoint_256.T_GrabPoint_256" :Option%204 "/Game/VRImmersiveHands/GrabSystem/Textures/T_GrabPoint_512.T_GrabPoint_512") :NewEnumerator1 (Utilities|Select :Index _pointsize :Option%200 0 :Option%201 "/Game/VRImmersiveHands/GrabSystem/Textures/T_RGrabPoint_64.T_RGrabPoint_64" :Option%202 "/Game/VRImmersiveHands/GrabSystem/Textures/T_RGrabPoint_128.T_RGrabPoint_128" :Option%203 "/Game/VRImmersiveHands/GrabSystem/Textures/T_RGrabPoint_256.T_RGrabPoint_256" :Option%204 "/Game/VRImmersiveHands/GrabSystem/Textures/T_RGrabPoint_512.T_RGrabPoint_512"))))
      (if (Variables|Grab|GetGlobalGrabPreview)
        (switch Utilities|FlowControl|Switch|SwitchonE_GrabbingDebug (.Debug (Utilities|Struct|BreakS_GrabPoints _array_element))
          (:NewEnumerator0
            (Grab|Preview|SpawnPreview (CallFunction|GetHandTransform (.RelativeTransformL (Utilities|Struct|BreakS_GrabPoints _array_element)) false _handscale) (.GrabAnim (Utilities|Struct|BreakS_GrabPoints _array_element)) "NewEnumerator0"))
          (:NewEnumerator1
            (Grab|Preview|SpawnPreview (CallFunction|GetHandTransform (.RelativeTransformL (Utilities|Struct|BreakS_GrabPoints _array_element)) true _handscale) (.GrabAnim (Utilities|Struct|BreakS_GrabPoints _array_element)) "NewEnumerator1"))
          (:NewEnumerator2
            (Grab|Preview|SpawnPreview (CallFunction|GetHandTransform (.RelativeTransformR (Utilities|Struct|BreakS_GrabPoints _array_element)) false _handscale) (.GrabAnim (Utilities|Struct|BreakS_GrabPoints _array_element)) "NewEnumerator1"))
          (:NewEnumerator3
            (Grab|Preview|SpawnPreview (CallFunction|GetHandTransform (.RelativeTransformR (Utilities|Struct|BreakS_GrabPoints _array_element)) true _handscale) (.GrabAnim (Utilities|Struct|BreakS_GrabPoints _array_element)) "NewEnumerator0"))
          (:NewEnumerator4
            (Grab|Preview|SpawnPreview (CallFunction|GetHandTransform (.RelativeTransformL (Utilities|Struct|BreakS_GrabPoints _array_element)) false _handscale) (.GrabAnim (Utilities|Struct|BreakS_GrabPoints _array_element)) "NewEnumerator0")
            (Grab|Preview|SpawnPreview (CallFunction|GetHandTransform (.RelativeTransformR (Utilities|Struct|BreakS_GrabPoints _array_element)) false _handscale) (.GrabAnim (Utilities|Struct|BreakS_GrabPoints _array_element)) "NewEnumerator1"))
          (:NewEnumerator5
            (Grab|Preview|SpawnPreview (CallFunction|GetHandTransform (.RelativeTransformL (Utilities|Struct|BreakS_GrabPoints _array_element)) true _handscale) (.GrabAnim (Utilities|Struct|BreakS_GrabPoints _array_element)) "NewEnumerator1")
            (Grab|Preview|SpawnPreview (CallFunction|GetHandTransform (.RelativeTransformR (Utilities|Struct|BreakS_GrabPoints _array_element)) false _handscale) (.GrabAnim (Utilities|Struct|BreakS_GrabPoints _array_element)) "NewEnumerator1"))
          (:NewEnumerator6
            (Grab|Preview|SpawnPreview (CallFunction|GetHandTransform (.RelativeTransformL (Utilities|Struct|BreakS_GrabPoints _array_element)) false _handscale) (.GrabAnim (Utilities|Struct|BreakS_GrabPoints _array_element)) "NewEnumerator0")
            (Grab|Preview|SpawnPreview (CallFunction|GetHandTransform (.RelativeTransformR (Utilities|Struct|BreakS_GrabPoints _array_element)) true _handscale) (.GrabAnim (Utilities|Struct|BreakS_GrabPoints _array_element)) "NewEnumerator0")))))))

(fn SpawnPreview
  (params (RelativeTransform :type Transform) (GrabAnim :type Anim%20Sequence%20Object%20Reference) (Hand :type E_Hand%20Enum :default "NewEnumerator0"))
  (bind _returnvalue (AddComponent|AddBPSCHandPreview (Actor|GetParentActor) false RelativeTransform))
  (Class|SkinnedMeshComponent|SetSkeletalMesh _returnvalue (Utilities|Select :Index Hand :NewEnumerator0 (Variables|Grab|Preview|GetPreviewSkMeshL) :NewEnumerator1 (Variables|Grab|Preview|GetPreviewSkMeshR)) true)
  (Variables|/Script/Engine.SkeletalMeshComponent|SetAnimationData _returnvalue (Utilities|Struct|MakeSingleAnimationPlayData GrabAnim false false 0.0 1.0)))

(fn Setup
  (params (Array :type Array%20of%20S%20Grab%20Points%20Structures))
  (Transformation|ResetRelativeTransform (Class|Actor|GetParentComponent))
  (for (_array_element _array_index) Array
    (bind _returnvalue (AddComponent|AddSphereComponent (Actor|GetAttachParentActor) true (Math|Transform|MakeTransform (.GrabPoint (Utilities|Struct|BreakS_GrabPoints _array_element)) "0, 0, 0" "1,1,1")))
    (Transformation|AttachComponentToComponent _returnvalue (Transformation|GetAttachParent (Variables|Default|GetDefaultSceneRoot)) "None" "KeepRelative" "KeepRelative" "KeepRelative" true)
    (CallFunction|SetTagValue (Variables|/Script/Engine.ActorComponent|GetComponentTags _returnvalue) "GrabType" (Utilities|Select :Index (.GrabType (Utilities|Struct|BreakS_GrabPoints _array_element)) :NewEnumerator0 "GP" :NewEnumerator1 "RGP"))
    (CallFunction|SetTagValue (Variables|/Script/Engine.ActorComponent|GetComponentTags _returnvalue) "GPIndex" (Utilities|String|StringToName (Utilities|String|ToString(Integer) _array_index)))
    (CallFunction|SetTagValue (Variables|/Script/Engine.ActorComponent|GetComponentTags _returnvalue) "LocalPriority" (Utilities|String|StringToName (Utilities|String|ToString(Integer) (.LocalGrabPriority (Utilities|Struct|BreakS_GrabPoints _array_element)))))
    (CallFunction|SetTagValue (Variables|/Script/Engine.ActorComponent|GetComponentTags _returnvalue) "OnlyGrabAsSecondary" (Utilities|String|StringToName (Utilities|String|ToString(Integer) (Math|Conversions|ToInteger(Boolean) (.OnlyGrabAsSecondary (Utilities|Struct|BreakS_GrabPoints _array_element)))))))
  (return))

(fn SetupGPC
  (bind _grabpoints (Variables|Grab|GetGrabPoints))
  (Setup|Setup _grabpoints)
  (return _grabpoints))

(fn SetupGSC
  (params (Array :type Array%20of%20S%20Grab%20Points%20Structures))
  (Setup|Setup Array)
  (return))