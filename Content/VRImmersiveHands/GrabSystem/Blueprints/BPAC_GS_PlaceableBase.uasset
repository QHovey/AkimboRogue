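; Actor component for the VR grab system that makes its owner a placement base with visual feedback for placing objects.
; It finds a tagged overlap shape, falling back to the first available, and an optional hidden base mesh.
; Events pulse the mesh or flash green or red for placement attempts, firing callbacks and recording success.
; Fake-timeline macros drive material parameters from separate channels of one vector curve.
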(event Custom|StartBasePulse
  ;[1 1 1] Pulse on Overlap
  (Variables|Default|GetMeshComponent
    (:then
      (if (Variables|ForInternalUse!|GetObjectPlaced)
        (CallFunction|StopBasePulse)
        (else
          (Default|CallOnPulseStart)
          (Rendering|SetVisibility (Variables|Default|GetMeshComponent) true false)
          (CallFunction|StopEfect)
          (if (not (Variables|ForInternalUse!|GetPlaying))
            (bind _subtractvalue (Utilities|PulseEfect)
              (:Subtract
                (Rendering|Material|SetScalarParameterValueonMaterials (Variables|Default|GetMeshComponent) "Subtract" _subtractvalue)))))))
    (:else)))

(event Custom|BasePlaceEfect
  (params (Correct :type Boolean))
  (bind _meshcomponent (Variables|Default|GetMeshComponent))
  ;[1 1 1] Efects
  (if Correct
    (Default|CallOnCorrectPlaceAttempt)
    (Variables|ForInternalUse!|SetObjectPlaced true)
    (Variables|Default|GetMeshComponent
      (:then
        (bind (_lerpvalue _colorvalue) (Utilities|BaseEfect "(R=0.000000,G=0.562433,B=0.181424,A=1.000000)")
          (:Lerp
            (Rendering|Material|SetScalarParameterValueonMaterials _meshcomponent "LerpMultiplier" _lerpvalue)
            (Rendering|Material|SetVectorParameterValueonMaterials _meshcomponent "Color" (Math|Conversions|ToVector(LinearColor) _colorvalue)))
          (:Finished
            (Default|CallOnPlaceComplete :!label _label)
            (CallFunction|StopBasePulse :!label _label_2)
            (CallFunction|DefaultParameters))))
      (:else
        (goto _label)))
    (else
      (Default|CallOnWrongPlaceAttempt)
      (Variables|Default|GetMeshComponent
        (:then
          (bind (_lerpvalue_2 _colorvalue_2) (Utilities|BaseEfect "(R=1.000000,G=0.082165,B=0.062269,A=1.000000)")
            (:Lerp
              (Rendering|Material|SetScalarParameterValueonMaterials _meshcomponent "LerpMultiplier" _lerpvalue_2)
              (Rendering|Material|SetVectorParameterValueonMaterials _meshcomponent "Color" (Math|Conversions|ToVector(LinearColor) _colorvalue_2)))
            (:Finished
              (goto _label_2))))
        (:else)))))

(event Custom|StopEfect
  (bind _meshcomponent (Variables|Default|GetMeshComponent))
  ;[1 1 1] Efects
  (Utilities|FlowControl|Sequence
    (:then_0
      (Utilities|BaseEfect "(R=0.000000,G=0.562433,B=0.181424,A=1.000000)") ; enters at Stop
    )
    (:then_1
      (Utilities|BaseEfect "(R=1.000000,G=0.082165,B=0.062269,A=1.000000)") ; enters at Stop
    )
    (:then_2
      (CallFunction|DefaultParameters))))

(event Custom|StopBasePulse
  ;[1 1 1] Pulse on Overlap
  (Variables|Default|GetMeshComponent
    (:then
      (Default|CallOnPulseEnd)
      (Rendering|SetVisibility (Variables|Default|GetMeshComponent) false false)
      (CallFunction|StopEfect)
      (Utilities|PulseEfect) ; enters at Stop
    )
    (:else)))

(event Custom|DefaultParameters
  ;[1 1 1] Efects
  (bind _meshcomponent (Variables|Default|GetMeshComponent)
    (:then
      (Rendering|Material|SetVectorParameterValueonMaterials _meshcomponent "Color" "1.000000,1.000000,1.000000")
      (Rendering|Material|SetScalarParameterValueonMaterials _meshcomponent "LerpMultiplier" 1.0))
    (:else)))

(event EventBeginPlay
  ;[1 1 1] Collision and base mesh
  (bind (_success _shapecomponent) (Utilities|TrytoFindCollision (Variables|Settings|GetCollisionTag)))
  (if _success
    (bind _output_get (Variables|ForInternalUse!|SetCollisionComponent _shapecomponent))
    (Collision|SetCollisionEnabled _output_get "QueryOnly")
    (Collision|SetCollisionObjectType _output_get "ECC_PhysicsBody")
    (Collision|SetCollisionResponsetoChannel _output_get "ECC_PhysicsBody" "ECR_Overlap")
    (Variables|/Script/Engine.PrimitiveComponent|SetbGenerateOverlapEvents _output_get true)
    (bind (_success_2 _meshcomponent) (CallFunction|InitializeComponent (Variables|Settings|GetBaseMeshTag)))
    (if _success_2
      (bind _output_get_2 (Variables|Default|SetMeshComponent _meshcomponent))
      (Collision|SetCollisionEnabled _output_get_2 "NoCollision")
      (Rendering|SetCastShadow _output_get_2 false)
      (Rendering|SetVisibility _output_get_2 false false)
      (if (Variables|Settings|GetOverrideBaseMeshMaterial)
        (Rendering|Material|SetMaterial _output_get_2 0 "/Game/VRImmersiveHands/GrabSystem/Materials/MI_Place.MI_Place"))
      (else
        (CallFunction|PrintWarning false "Couldn't find a mesh for Base Mesh. Placeable Base can work without Base Mesh. This is just a reminder. ")))
    (else
      (CallFunction|DestroyComponent "Can't find a Collision Component."))))

(fn FindCollisioninOwner
  (params (Tag :type Name%20%28by%20ref%29))
  (LocalVariables|SetShape 0)
  (bind _array_element (Utilities|Array|ForEachLoopwithBreak (Actor|GetComponentsByClass (Components|GetOwner) "/Script/Engine.ShapeComponent") :!label _label)
    (:LoopBody
      (if (Utilities|Array|ContainsItem (Variables|/Script/Engine.ActorComponent|GetComponentTags _array_element) Tag)
        (LocalVariables|SetShape _array_element)
        (goto _label Break)))
    (:Completed
      (bind _shape (LocalVariables|GetShape)
        (:then
          (return true _shape))
        (:else
          (return false 0))))))

(fn GetFirstCollisioninOwner
  (bind _output_get (LocalVariables|SetShape (Actor|GetComponentbyClass (Components|GetOwner) "/Script/Engine.ShapeComponent")))
  (Utilities|IsValid _output_get
    (:Is%20Valid
      (return true _output_get))
    (:Is%20Not%20Valid
      (return false 0))))

(fn TrytoFindCollision
  (params (Tag :type Name))
  (bind (_success _shapecomponent) (Core|FindCollisioninOwner Tag))
  (if _success
    (return true _shapecomponent)
    (else
      (bind (_success_2 _shapecomponent_2) (Core|GetFirstCollisioninOwner))
      (if _success_2
        (CallFunction|PrintWarning false (Utilities|String|Append "Couldn't find a collision component with the following tag, --- " (Utilities|String|ToString(Name) Tag) " ---. " (Utilities|GetObjectName _shapecomponent_2) " will be used instead."))
        (return true _shapecomponent_2)
        (else
          (return false 0))))))