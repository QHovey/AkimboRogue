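; Grab System component that plays an impact sound when the grabbable's physics mesh hits something.
; It binds to hits once the Grabbing Core initializes, and destroys itself if the core is destroyed or hit events are disabled.
; Squared impulse change filters hits: large changes play immediately, moderate ones are throttled by a delayed DoOnce, small ones are ignored.
; Hits are briefly muted after setup and when physics simulation starts.
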(event Custom|PhysicsUpdated
  (params (Simulating :type Boolean))
  ;[1 1 1] Find Grabbing Core and wait for it to be initialized. If its destroyed, destroy this component as well.
  (if Simulating
    (CallFunction|JustSpawned)))

(event Custom|OnDestroyEvent
  ;[1 1 1] Find Grabbing Core and wait for it to be initialized. If its destroyed, destroy this component as well.
  (CallFunction|DestroyComponent "BPAC_GS_Core is being destroyed."))

(event Custom|Reset
  ;[1 1 1] Play sound in Hit
  (Utilities|FlowControl|DoOnce false) ; enters at Reset
)

(event Custom|JustSpawned
  ;[1 1 1] Quick Fix for playing sound on spawn
  (Variables|ForInternalUse!|SetSpawnFix true)
  (Utilities|FlowControl|Delay 0.5)
  (Variables|ForInternalUse!|SetSpawnFix false))

(event Custom|Setup
  (bind _grabbingcore (Variables|Default|GetGrabbingCore))
  (bind _meshcomponent (Variables|/Game/VRImmersiveHands/GrabSystem/Blueprints/BPAC_GS_Common.BPAC_GS_Common_C|GetMeshComponent _grabbingcore))
  ;[1 1 1] Setup
  (if (Utilities|Struct|BreakBodyInstance (Variables|/Script/Engine.PrimitiveComponent|GetBodyInstance _meshcomponent))
    (Collision|AssignOnComponentHit _meshcomponent (delegate Custom|On%20Hit))
    (CallFunction|JustSpawned)
    (else
      (CallFunction|DestroyComponent "Simulation Generates Hit Events is not set to TRUE! This can't be set with BP, so it has to be set manually from collision section."))))

(event Custom|On%20Hit
  (params (HitComponent :type Primitive%20Component%20Object%20Reference) (OtherActor :type Actor%20Object%20Reference) (OtherComp :type Primitive%20Component%20Object%20Reference) (NormalImpulse :type Vector) (Hit :type Hit%20Result%20Structure%20%28by%20ref%29))
  ;[1 1 1] Play sound in Hit
  (if (not (Variables|ForInternalUse!|GetSpawnFix))
    (if (> (Math|Vector|VectorLengthSquared NormalImpulse) 1.0)
      (Utilities|ComparetoTwoFloats (Class|KismetMathLibrary|VectorDistanceSquared NormalImpulse (Variables|ForInternalUse!|GetLastImpact)) 1.0 2.0 ; If the impact change is above Max, its problaly a totally new impact. So go right ahead and play the sound. \nIf the impact change is between Min and Max, it problaly fell down and its damping. So wait 0.5 seconds to play the sound to filter Event Hit a bit.  \nIf the impact change is below Min, its problaly beign dragged across or almost settled. So dont do anything.
        (:>
          (CallFunction|Reset))
        (:<=>
          _))
      (Variables|ForInternalUse!|SetLastImpact NormalImpulse)
      (Utilities|FlowControl|DoOnce false
        (:Completed
          (Audio|PlaySoundatLocation (Variables|Settings|GetSound) (.Location (Collision|BreakHitResult Hit)) "0, 0, 0" 1.0 1.0 0.0 0 0 0)
          (Utilities|FlowControl|RetriggerableDelay 0.5)
          (CallFunction|Reset))))))

(event EventBeginPlay
  (bind _grabbingcore (Variables|Default|GetGrabbingCore))
  ;[1 1 1] Find Grabbing Core and wait for it to be initialized. If its destroyed, destroy this component as well.
  (bind (_success _grabbingcore_2) (CallFunction|GetGrabbingCore))
  (if _success
    (EventDispatchers|AssignOnDestroy _grabbingcore_2 (delegate Custom|OnDestroyEvent))
    (EventDispatchers|AssignPhysicsUpdated _grabbingcore (delegate Custom|PhysicsUpdated))
    (if (Variables|/Game/VRImmersiveHands/GrabSystem/Blueprints/BPAC_GS_Core.BPAC_GS_Core_C|GetInitialized _grabbingcore_2)
      (CallFunction|Setup)
      (else
        (EventDispatchers|AssignCoreInitialized _grabbingcore (delegate Custom|Setup))))))