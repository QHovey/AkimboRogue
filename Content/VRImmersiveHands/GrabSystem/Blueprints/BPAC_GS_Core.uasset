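; VR grab-system core component that makes its owner's tagged static mesh a grabbable, optionally physics-simulated object.
; On BeginPlay it configures the mesh and exchanges grab points with a child constructor actor, which it then destroys.
; Normal grabs attach and ease the mesh to the hand, while reverse grabs return mesh, animation and transform to the caller.
; It also gates grabs by GrabType tags, handles hand swaps and restores physics on drop.
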(event Custom|Dropped
  ;[1 1 1] Start Physics and Detach
  (Default|CallOnDropped))

(event Custom|Drop
  ;[1 1 1] Start Physics and Detach
  (Default|CallOnDrop)
  (Variables|ForInternalUse!|SetGrabbed false)
  (CallFunction|StopLerp) ; You might want to Drop the object while its lerping to hand. \nSo we Stop Lerp to make sure its dropping properly.
  (Settings|UpdatePhysics)
  (Transformation|DetachFromComponent (Variables|Default|GetMeshComponent) "KeepWorld" "KeepWorld" "KeepWorld" true)
  (CallFunction|Dropped))

(event Custom|LerpToHand
  (params (Parent :type Scene%20Component%20Object%20Reference) (To :type Transform) (TravelTime :type Float%20%28single-precision%29))
  (bind _meshcomponent (Variables|Default|GetMeshComponent))
  (bind _meshcomponent_2 (Variables|Default|GetMeshComponent))
  ;[1 1 1] Lerp to Hand for Smooth Grabbing
  (Variables|ForInternalUse!|SetTempTo To)
  (Variables|ForInternalUse!|SetLerping true)
  (Settings|UpdatePhysics)
  (Transformation|AttachComponentToComponent _meshcomponent Parent "None" "KeepWorld" "KeepWorld" "KeepWorld" true)
  (Variables|ForInternalUse!|SetTempFrom (Transformation|GetRelativeTransform _meshcomponent))
  (bind _updatevalue (Utilities|FakeTimeline 0.02 TravelTime)
    (:Update
      (Transformation|SetRelativeTransform _meshcomponent_2 (Math|Transform|MakeTransform (.location (Math|Transform|Lerp(Transform) (Variables|ForInternalUse!|GetTempFrom) (Variables|ForInternalUse!|GetTempTo) (Math|Interpolation|Ease "SinusoidalInOut" (Math|Float|MapRangeClamped _updatevalue 0.0 TravelTime 0.0 1.0) 0.0 1.0))) (.rotation (Math|Transform|Lerp(Transform) (Variables|ForInternalUse!|GetTempFrom) (Variables|ForInternalUse!|GetTempTo) (Math|Interpolation|Ease "SinusoidalInOut" (Math|Float|MapRangeClamped _updatevalue 0.0 TravelTime 0.0 1.0) 0.0 1.0))) (Variables|/Script/Engine.SceneComponent|GetRelativeScale3D _meshcomponent_2)) false false))
    (:Finished
      (Variables|ForInternalUse!|SetLerping false :!label _label))
    (:Stopped
      (goto _label))))

(event Custom|StopLerp
  (bind _meshcomponent (Variables|Default|GetMeshComponent))
  ;[1 1 1] Lerp to Hand for Smooth Grabbing
  (Utilities|FakeTimeline 0.02 (stale Custom|LerpToHand TravelTime)) ; enters at Stop
)

(event EventBeginPlay
  ;[1 1 1] Find Static Mesh
  (bind (_success _meshcomponent) (CallFunction|InitializeComponent (Variables|Default|GetMeshComponentTag)))
  (if _success
    (bind _output_get (Variables|Default|SetMeshComponent _meshcomponent))
    (Transformation|SetMobility _output_get "Movable")
    (Collision|SetCollisionEnabled _output_get "QueryAndPhysics")
    (Collision|SetCollisionObjectType _output_get "ECC_PhysicsBody")
    (Collision|SetCollisionResponsetoAllChannels _output_get "ECR_Block")
    (Variables|/Script/Engine.PrimitiveComponent|SetbGenerateOverlapEvents _output_get true)
    ;[1 1 1] Find Components
    (Grab|GrabPoint|SetupGrabPoint)
    ;[1 1 1] Setup
    (Settings|SetSettings (Variables|Settings|GetCanInteract) (Variables|Settings|GetSimulatePhysics))
    (Default|CallCoreInitialized)
    (Variables|ForInternalUse!|SetInitialized true)
    (else
      (CallFunction|DestroyComponent "Can't find the Static Mesh."))))

(fn SetSettings
  (params (CanInteract :type Boolean) (SimulatePhysics :type Boolean))
  (Variables|Settings|SetCanInteract CanInteract)
  (Settings|SetPhysics SimulatePhysics))

(fn SetPhysics
  (params (SimulatePhysics :type Boolean))
  (Variables|Settings|SetSimulatePhysics SimulatePhysics)
  (Settings|UpdatePhysics))

(fn UpdatePhysics
  (bind _meshcomponent (Variables|Default|GetMeshComponent))
  (if (and (Variables|Settings|GetSimulatePhysics) (not (Variables|ForInternalUse!|GetGrabbed)))
    (Physics|SetSimulatePhysics _meshcomponent true)
    (Default|CallPhysicsUpdated true)
    (return true)
    (else
      (Physics|SetSimulatePhysics _meshcomponent false)
      (Default|CallPhysicsUpdated false)
      (return false))))

(fn SetupGrabPoint
  (LocalVariables|SetChild 0)
  (for _array_element (Actor|GetAllChildActors (Components|GetOwner) false)
    (bind _asbp_grab_point_constructor (Utilities|Casting|CastToBP_GrabPointConstructor _array_element))
    (LocalVariables|GetChild
      (:then
        (Actor|DestroyActor _array_element)
        (CallFunction|PrintWarning false (Utilities|String|Append "Found more than 1 Grab Point Contructor! Destroying ---" (Utilities|GetDisplayName _array_element) "---")))
      (:else
        (LocalVariables|SetChild _asbp_grab_point_constructor))))
  (bind _child (LocalVariables|GetChild)
    (:then
      (if (Utilities|Array|IsValidIndex (Variables|Settings|GetGrabPoints))
        (Default|SetupGSC _child (Variables|Settings|GetGrabPoints))
        (else
          (bind _grabpoints (Default|SetupGPC _child))
          (Variables|Settings|SetGrabPoints _grabpoints)))
      (Actor|DestroyActor _child)
      (return true))
    (:else
      (return false))))

(fn GrabPointGrab
  (params (Root :type Scene%20Component%20Object%20Reference) (Hand :type E_Hand%20Enum :default "NewEnumerator0") (Point :type Integer))
  (bind _grabpoints (Variables|Settings|GetGrabPoints))
  (bind _output (Utilities|Array|Get(acopy) _grabpoints Point))
  (bind (_relativetransforml _relativetransformr _grabanim) (Utilities|Struct|BreakS_GrabPoints _output))
  (Grab|Utilities|HandleSwap Hand)
  (Variables|ForInternalUse!|SetHand Hand)
  (Variables|ForInternalUse!|SetGrabbed true)
  (CallFunction|LerptoHand Root (Utilities|Select :Index (Variables|ForInternalUse!|GetHand) :NewEnumerator0 _relativetransforml :NewEnumerator1 _relativetransformr) (Variables|Settings|GetTravelTime))
  (Default|CallOnGrabbed "NewEnumerator0")
  (return _grabanim))

(fn ReverseGrabPointGrab
  (params (Hand :type E_Hand%20Enum :default "NewEnumerator0") (Point :type Integer))
  (bind _grabpoints (Variables|Settings|GetGrabPoints))
  (bind _output (Utilities|Array|Get(acopy) _grabpoints Point))
  (bind (_relativetransforml _relativetransformr _grabanim) (Utilities|Struct|BreakS_GrabPoints _output))
  (Variables|ForInternalUse!|SetGrabbed true)
  (Default|CallOnGrabbed "NewEnumerator1")
  (return _grabanim (Variables|Default|GetMeshComponent) (Utilities|Select :Index Hand :NewEnumerator0 _relativetransforml :NewEnumerator1 _relativetransformr)))

(fn CanbeGrabbed?
  (params (Tags :type Array%20of%20Names))
  (bind _grabbed (Variables|ForInternalUse!|GetGrabbed))
  (if (and (Variables|Settings|GetCanInteract) (Math|Boolean|NORBoolean (Variables|ForInternalUse!|GetBlock) (Variables|ForInternalUse!|GetLerping)))
    (switch name (.Value (CallFunction|GetTagValue Tags "GrabType"))
      (:Default
        _)
      (:GP
        (if _grabbed
          (if (Variables|Settings|GetAllowHandSwap)
            (return true (Variables|Settings|GetGrabPriority))
            (else
              _))
          (else
            (return true (Variables|Settings|GetGrabPriority)))))
      (:RGP
        (if (Math|Conversions|ToBoolean(Integer) (Math|Conversions|ToInteger(Byte) (Utilities|String|ToString(Name) (.Value (CallFunction|GetTagValue Tags "OnlyGrabAsSecondary")))))
          (if _grabbed
            (return true (Variables|Settings|GetGrabPriority))
            (else
              _))
          (else
            (return true (Variables|Settings|GetGrabPriority)))))))
  (return false 0))

(fn ExternalBlock
  (params (Block :type Boolean))
  (Variables|ForInternalUse!|SetBlock Block))

(fn HandleSwap
  (params (Hand :type E_Hand%20Enum :default "NewEnumerator0"))
  (if (and (Utilities|Enum|NotEqual(Enum) Hand (Variables|ForInternalUse!|GetHand)) (Variables|ForInternalUse!|GetGrabbed))
    (Default|ForceRelease (.AsBP%20HAC%20GS (Utilities|Casting|CastToBP_HAC_GS (.HAC (CallFunction|GetHAC (Variables|ForInternalUse!|GetHand))))))))