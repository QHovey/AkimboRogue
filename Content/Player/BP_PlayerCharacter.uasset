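; Player character playable in VR or first person, with two grab-capable hands, a teleporter per motion controller and test weapons equipped on spawn.
; Switching VR mode re-parents the hands to motion controllers or camera-front anchors and reconfigures camera and rotation.
; Thumbsticks, or middle mouse outside VR, drive teleporters; teleporting fades the camera and briefly disables capsule collision to skip blocking checks.
; A GAS cooldown effect follows each teleport, gated by a gameplay tag.
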(event Custom|ExecuteTeleportation
  (params (Teleporter :type Teleporter%20Object%20Reference))
  (bind (_location _rotation) (Default|GetTeleportDestination Teleporter))
  (bind _fadeoutduration (Variables|Default|GetFadeOutDuration))
  (bind _abilitysystemcomponent (Variables|Default|GetAbilitySystemComponent))
  ;[0 0 0] Handle Teleportation
  (if (not (Variables|Default|GetIsTeleporting))
    (if (Variables|/Game/Player/Teleporter.Teleporter_C|GetIsValidTeleportDestination Teleporter)
      (Variables|Default|SetIsTeleporting true)
      (CameraFades|StartCameraFade (Game|GetPlayerCameraManager 0) 0.0 1.0 _fadeoutduration (Variables|Default|GetTeleportFadeColor) false true)
      (Utilities|FlowControl|Delay _fadeoutduration)
      (Default|DisableTeleporter Teleporter)
      ;;[0.2448 0.2448 0.2448] Semi Hack: Disable Collision before the Teleport call to skip blocking Geo checks. We already made sure the destination isn't blocked when determining the location.
      (Collision|SetCollisionEnabled (Variables|Default|GetCapsuleComponent) "NoCollision")
      (Transformation|Teleport _location _rotation)
      (Collision|SetCollisionEnabled (Variables|Default|GetCapsuleComponent) "QueryOnly")
      (CameraFades|StartCameraFade (Game|GetPlayerCameraManager 0) 1.0 0.0 (Variables|Default|GetFadeInDuration) (Variables|Default|GetTeleportFadeColor) false false)
      (Variables|Default|SetIsTeleporting false)
      (GameplayEffects|ApplyGameplayEffectSpecToSelf _abilitysystemcomponent (GameplayEffects|MakeOutgoingSpec :self _abilitysystemcomponent :GameplayEffectClass "/Game/GameplayEffects/Cooldowns/GE_CooldownTeleport.GE_CooldownTeleport_C" :Level 1.0))
      (else
        (Default|DisableTeleporter Teleporter)))))

(event EventTick
  (params (DeltaSeconds :type Float%20%28single-precision%29)))

(event EventOnVRModeChanged
  (params (VREnabled :type Boolean))
  (if VREnabled
    ;[1 1 1] VRMode - Hands attach to motion controllers
    (Transformation|AttachComponentToComponent (Variables|HAC_GS|GetLeftHAC_GS) (Variables|Default|GetL_MotionController) "None" "SnapToTarget" "SnapToTarget" "SnapToTarget" true)
    (Transformation|AttachComponentToComponent (Variables|HAC_GS|GetRightHAC_GS) (Variables|Default|GetR_MotionController) "None" "SnapToTarget" "SnapToTarget" "SnapToTarget" true)
    (Variables|/Script/Engine.CameraComponent|SetbLockToHmd (Variables|Default|GetCameraComponent) true)
    (Variables|/Script/Engine.CameraComponent|SetbUsePawnControlRotation (Variables|Default|GetCameraComponent) false)
    (Variables|Default|SetbUseControllerRotationYaw false)
    (CallFunction|EnableVR true 1.0)
    (else
      ;[1 1 1] FirstPersonMode - Hands attach to static positions in front of camera
      (Transformation|AttachComponentToComponent (Variables|HAC_GS|GetLeftHAC_GS) (Variables|Default|GetL_FPHandPos) "None" "SnapToTarget" "SnapToTarget" "SnapToTarget" true)
      (Transformation|AttachComponentToComponent (Variables|HAC_GS|GetRightHAC_GS) (Variables|Default|GetR_FPHandPos) "None" "SnapToTarget" "SnapToTarget" "SnapToTarget" true)
      (Variables|/Script/Engine.CameraComponent|SetbLockToHmd (Variables|Default|GetCameraComponent) false)
      (Variables|/Script/Engine.CameraComponent|SetbUsePawnControlRotation (Variables|Default|GetCameraComponent) true)
      (Variables|Default|SetbUseControllerRotationYaw true)
      (Transformation|SetRelativeLocation (Variables|Default|GetCameraComponent) "-39.560001, 0,160.000000" false false)
      (Transformation|SetRelativeRotation (Variables|Default|GetCameraComponent) "0, 0, 0" false false)
      (CallFunction|EnableVR false 1.0))))

(event EventBeginPlay
  (bind _returnvalue (Math|Transform|MakeTransform "0, 0, 0"))
  (Utilities|FlowControl|Sequence
    (:then_0
      ;[0 1 0.1203] Spawn HACs
      (bind (_lefthac _righthac) (Default|SpawnHACGSs (Variables|HAC_GS|GetBPAC_HAC_GS) (Variables|HAC_GS|GetSettings) (select (Variables|Default|GetIsVR) (Variables|Default|GetL_MotionController) (Variables|Default|GetL_FPHandPos)) (select (Variables|Default|GetIsVR) (Variables|Default|GetR_MotionController) (Variables|Default|GetR_FPHandPos))))
      (Variables|HAC_GS|SetLeftHAC_GS _lefthac)
      (Variables|HAC_GS|SetRightHAC_GS _righthac))
    (:then_1
      (Class|HeadMountedDisplayFunctionLibrary|SetTrackingOrigin "Floor") ; Windows (Oculus / Vive)
    )
    (:then_2
      ;[1 1 1] Create Teleporters
      (bind _returnvalue_2 (Game|SpawnActorfromClass "/Game/Player/Teleporter.Teleporter_C" (Math|Transform|MakeTransform "0, 0, 0") "Undefined" self "Left" 0))
      (bind _output_get (Variables|Default|SetLeftTeleporter _returnvalue_2))
      (Transformation|AttachComponentToComponent _output_get (Variables|Default|GetL_MotionController) "None" "SnapToTarget" "SnapToTarget" "KeepRelative" true)
      (bind _returnvalue_3 (Game|SpawnActorfromClass "/Game/Player/Teleporter.Teleporter_C" (Math|Transform|MakeTransform "0, 0, 0") "Undefined" self "Right" 0))
      (bind _output_get_2 (Variables|Default|SetRightTeleporter _returnvalue_3))
      (Transformation|AttachComponentToComponent _output_get_2 (Variables|Default|GetR_MotionController) "None" "SnapToTarget" "SnapToTarget" "KeepRelative" true))
    (:then_3
      (bind _returnvalue_4 (Game|SpawnActorfromClass "/Game/Weapons/TestPlayerWeapon/TestPlayerWeapon.TestPlayerWeapon_C" _returnvalue "Undefined" 0 0))
      (Class|AkimboCharacter|EquipLeftWeapon _returnvalue_4)
      (bind _returnvalue_5 (Game|SpawnActorfromClass "/Game/Weapons/TestPlayerWeapon/TestPlayerWeapon.TestPlayerWeapon_C" _returnvalue "Undefined" 0 0))
      (Class|AkimboCharacter|EquipRightWeapon _returnvalue_5))))

(event Collision|EventActorBeginOverlap
  (params (OtherActor :type Actor%20Object%20Reference)))

(event EventOnRightWeaponEquipped
  (params (Weapon :type Akimbo%20Weapon%20Object%20Reference))
  (bind _gs_core (Class|BPIGSCoreOwner|GetGSCore(Message) Weapon))
  (Utilities|IsValid _gs_core
    (:Is%20Valid
      (Default|ForceGrab (Variables|HAC_GS|GetRightHAC_GS) _gs_core "NewEnumerator1")
      (Input|EnableInput Weapon (Game|GetPlayerController 0)))))

(event EventOnLeftWeaponEquipped
  (params (Weapon :type Akimbo%20Weapon%20Object%20Reference))
  (bind _gs_core (Class|BPIGSCoreOwner|GetGSCore(Message) Weapon))
  (Utilities|IsValid _gs_core
    (:Is%20Valid
      (Default|ForceGrab (Variables|HAC_GS|GetLeftHAC_GS) _gs_core "NewEnumerator0")
      (Input|EnableInput Weapon (Game|GetPlayerController 0)))))

(event Input|AxisEvents|InputAxisMotionControllerThumbLeft_Y
  (params (AxisValue :type Float%20%28single-precision%29))
  ;[1 1 1] Teleportation Input
  ;;[1 1 1] VR Teleporter, the actual input used in the final game. Uses stick direction to aim location rotation.
  (if (Variables|Default|GetIsVR)
    (CallFunction|HandleTeleportInput (Variables|Default|GetLeftTeleporter) (stale Input|AxisEvents|InputAxisMotionControllerThumbLeft_X AxisValue) AxisValue)))

(event Input|AxisEvents|InputAxisMotionControllerThumbLeft_X
  (params (AxisValue :type Float%20%28single-precision%29))
  ;[1 1 1] Teleportation Input
  ;;[1 1 1] VR Teleporter, the actual input used in the final game. Uses stick direction to aim location rotation.
  (if (Variables|Default|GetIsVR)
    (CallFunction|HandleTeleportInput (Variables|Default|GetLeftTeleporter) AxisValue (stale Input|AxisEvents|InputAxisMotionControllerThumbLeft_Y AxisValue))))

(event Input|AxisEvents|InputAxisMotionControllerThumbRight_X
  (params (AxisValue :type Float%20%28single-precision%29))
  ;[1 1 1] Teleportation Input
  ;;[1 1 1] VR Teleporter, the actual input used in the final game. Uses stick direction to aim location rotation.
  (if (Variables|Default|GetIsVR)
    (CallFunction|HandleTeleportInput (Variables|Default|GetRightTeleporter) AxisValue (stale Input|AxisEvents|InputAxisMotionControllerThumbRight_Y AxisValue))))

(event Input|AxisEvents|InputAxisMotionControllerThumbRight_Y
  (params (AxisValue :type Float%20%28single-precision%29))
  ;[1 1 1] Teleportation Input
  ;;[1 1 1] VR Teleporter, the actual input used in the final game. Uses stick direction to aim location rotation.
  (if (Variables|Default|GetIsVR)
    (CallFunction|HandleTeleportInput (Variables|Default|GetRightTeleporter) (stale Input|AxisEvents|InputAxisMotionControllerThumbRight_X AxisValue) AxisValue)))

(event Input|MouseEvents|MiddleMouseButton
  (params (Key :type Key%20Structure :default "None"))
  (bind _rightteleporter (Variables|Default|GetRightTeleporter))
  ;[1 1 1] Teleportation Input
  ;;[1 1 1] Mouse input for Non-VR debugging. Simply aims teleporter forward from RIght Hand
  (:Pressed
    (if (not (Variables|Default|GetIsVR))
      (CallFunction|HandleTeleportInput _rightteleporter 0.0 1.0)))
  (:Released
    (if (not (Variables|Default|GetIsVR))
      (CallFunction|HandleTeleportInput _rightteleporter 0.0 0.0))))

(fn ConstructionScript)

(fn HandleTeleportInput
  (params (Teleporter :type Teleporter%20Object%20Reference) (InputX :type Float%20%28single-precision%29) (InputY :type Float%20%28single-precision%29))
  (bind _executeteleport (Default|UpdateTeleporterfromInput Teleporter InputX InputY))
  (if (and _executeteleport (not (GameplayTags|HasMatchingGameplayTag (Variables|Default|GetAbilitySystemComponent) "(TagName=\"Ability.Teleport\")")))
    (CallFunction|ExecuteTeleportation Teleporter)
    (Development|PrintString "Hello")))